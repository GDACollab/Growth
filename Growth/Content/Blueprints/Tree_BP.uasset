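; Tree Blueprint that grows a single root at a random spot on its sprite when play begins.
; BeginPlay spawns a half-scale Root_BP actor, then picks one of three sockets on TreeSprite at random: left, middle or right.
; The new root's scene root attaches to the chosen socket, and the construction script is empty.
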(event `self.ReceiveBeginPlay`
  ;[1 1 1] Randomly generate root sprite on one of three sockets
  (bind _returnvalue (`|SpawnActorFromClass` "/Game/Blueprints/Root_BP.Root_BP_C" (`KismetMathLibrary.MakeTransform` (0.0 5.0 -15.0) (struct) (0.5 0.5 0.5)) "AdjustIfPossibleButDontSpawnIfColliding" "OverrideRootScale"))
  (switch `int` (`KismetMathLibrary.RandomInteger` 3)
    (:`0`
      (bind _defaultsceneroot (`/Game/Blueprints/Root_BP.DefaultSceneRoot` _returnvalue))
      (`SceneComponent.K2_AttachTo` _defaultsceneroot (`self.Tree_Sprite`) "LeftRoot" "KeepRelativeOffset" true))
    (:`1`
      (`SceneComponent.K2_AttachTo` _defaultsceneroot (`self.Tree_Sprite`) "MidRoot" "KeepRelativeOffset" true))
    (:`2`
      (`SceneComponent.K2_AttachTo` _defaultsceneroot (`self.Tree_Sprite`) "RightRoot" "KeepRelativeOffset" true))))

(fn `UserConstructionScript`)