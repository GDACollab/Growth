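; Player controller that edge-scrolls the main GrowthCamera with the mouse.
; On BeginPlay it shows the cursor, enables click events and caches the player character as a GrowthCamera.
; Each Tick, IsMouseLeft and IsMouseRight test whether the cursor sits in the outer tenth of the viewport width on either side, calling Sweep on the camera with a negative or positive direction accordingly.
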(event `self.ReceiveBeginPlay`
  ;[1 1 1] Get reference to Main Camera
  (set `self.bShowMouseCursor` true)
  (bind _asgrowth_camera (cast `/Game/Blueprints/Player/GrowthCamera` (`GameplayStatics.GetPlayerCharacter` 0)))
  (set `self.GrowthCamera` _asgrowth_camera)
  (set `self.bEnableClickEvents` true))

(event `self.ReceiveTick`
  (params (DeltaSeconds :type "Float (single-precision)"))
  (bind _growthcamera (`self.GrowthCamera`))
  ;[1 1 1] Move Main Camera based on mouse location
  (`|ExecutionSequence`
    (:`then_0`
      (bind _ismouseleft (`self.IsMouseLeft`))
      (if _ismouseleft
        (`/Game/Blueprints/Player/GrowthCamera.Sweep` _growthcamera -1.0)))
    (:`then_1`
      (bind _ismouseright (`self.IsMouseRight`))
      (if _ismouseright
        (`/Game/Blueprints/Player/GrowthCamera.Sweep` _growthcamera 1.0)))))

(fn `IsMouseLeft`
  (returns (isMouseLeft :type Boolean))
  (return (and (<= (`self.GetMousePosition`) (`KismetMathLibrary.Conv_IntToDouble` (/ (`self.GetViewportSize`) 10))) (> (`self.GetMousePosition`) 0.0))))

(fn `IsMouseRight`
  (returns (isMouseRight :type Boolean))
  (return (and (<= (`self.GetMousePosition`) (`KismetMathLibrary.Conv_IntToDouble` (`self.GetViewportSize`))) (>= (`self.GetMousePosition`) (- (`KismetMathLibrary.Conv_IntToDouble` (`self.GetViewportSize`)) (/ (`KismetMathLibrary.Conv_IntToDouble` (`self.GetViewportSize`)) 10.0))))))

(fn `UserConstructionScript`)