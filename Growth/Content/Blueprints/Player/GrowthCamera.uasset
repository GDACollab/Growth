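; Player camera pawn that pans along world X, owns the HUD, resource bars and pause menu, and tracks growth resources.
; Each tick drains water, air and sunlight; energy rises below max while all three remain, otherwise drains.
; IncrementResource adds fixed amounts to a chosen resource, and updates write directly to Bars.
; Depletion scales with global time dilation but not delta time, energy gain with neither, and panning input compensates for dilation.
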(event `self.ReceiveBeginPlay`
  ;[1 0.2845 0.6013] Get References to UI
  (bind _returnvalue (`|CreateWidget` "/Game/UserInterface/Pause.Pause_C"))
  (set `self.Pause Menu` _returnvalue)
  (bind _returnvalue_2 (`|CreateWidget` "/Game/UserInterface/HUD.HUD_C"))
  (bind _output_get (set `self.HUD` _returnvalue_2))
  (bind _returnvalue_3 (`|CreateWidget` "/Game/UserInterface/Bars.Bars_C"))
  (bind _output_get_2 (set `self.Bars` _returnvalue_3))
  (`UserWidget.AddToViewport` _output_get_2 0)
  (`UserWidget.AddToViewport` _output_get 0))

(event `Sweep`
  (params (ScaleValue :type "Float (double-precision)"))
  ;[1 1 1] Move Camera
  (`self.AddMovementInput` (1.0 0.0 0.0) (* ScaleValue (/ 1.0 (`GameplayStatics.GetGlobalTimeDilation`)))))

(event `InputAction|Pause` :paused true
  (params (Key :type "Key Structure" :default "AnyKey"))
  ;[1 1 1] Pause and Unpause with Tab
  (:`Pressed`
    (if (`GameplayStatics.IsGamePaused`)
      (`self.Unpause`)
      (else
        (`self.Pause`)))))

(event `self.ReceiveTick`
  (params (DeltaSeconds :type "Float (single-precision)"))
  ;[1 1 1] Constantly Update Energy
  (`self.UpdateEnergy`)
  (`self.UpdateWater`)
  (`self.UpdateAir`)
  (`self.UpdateSunlight`))

(event `InputAxis|MoveRight`
  (params (AxisValue :type "Float (single-precision)"))
  ;[1 1 1] Handle Keyboard Input
  (`self.Sweep` AxisValue))

(fn `IncrementResource`
  (params (ResourceType :type "/Game/Blueprints/Enum_ResourceType Enum"))
  (bind _currentair (`self.CurrentAir`))
  (bind _maxair (`self.MaxAir`))
  (bind _currentwater (`self.CurrentWater`))
  (bind _maxwater (`self.MaxWater`))
  (bind _currentsunlight (`self.CurrentSunlight`))
  (bind _maxsunlight (`self.MaxSunlight`))
  (switch `/Game/Blueprints/Enum_ResourceType` ResourceType
    (:`NewEnumerator0`
      ;[0 0.2211 1] Increment Water Resource
      (if (< (`self.CurrentWater`) (`self.MaxWater`))
        (set `self.CurrentWater` (+ (`self.CurrentWater`) 10.0))
        (set `/Game/UserInterface/Bars.WaterPercentage` (/ _currentwater _maxwater) (`self.Bars`))
        (set `/Game/UserInterface/Bars.WaterText` (`KismetStringLibrary.Concat_StrStr` (`KismetStringLibrary.Conv_IntToString` (`KismetMathLibrary.FFloor` _currentwater)) "/" (`KismetStringLibrary.Conv_IntToString` (`KismetMathLibrary.FFloor` _maxwater))) (`self.Bars`))))
    (:`NewEnumerator1`
      ;[0 0.8813 1] Increment Air Resource
      (if (< (`self.CurrentAir`) (`self.MaxAir`))
        (set `self.CurrentAir` (+ (`self.CurrentAir`) 10.0))
        (set `/Game/UserInterface/Bars.AirPercentage` (/ _currentair _maxair) (`self.Bars`))
        (set `/Game/UserInterface/Bars.AirText` (`KismetStringLibrary.Concat_StrStr` (`KismetStringLibrary.Conv_IntToString` (`KismetMathLibrary.FFloor` _currentair)) "/" (`KismetStringLibrary.Conv_IntToString` (`KismetMathLibrary.FFloor` _maxair))) (`self.Bars`))))
    (:`NewEnumerator2`
      ;[1 0.8781 0.0519] Increment Sunlight Resource
      (if (< (`self.CurrentSunlight`) (`self.MaxSunlight`))
        (set `self.CurrentSunlight` (+ (`self.CurrentSunlight`) 10.0))
        (set `/Game/UserInterface/Bars.SunlightPercentage` (/ _currentsunlight _maxsunlight) (`self.Bars`))
        (set `/Game/UserInterface/Bars.SunlightText` (`KismetStringLibrary.Concat_StrStr` (`KismetStringLibrary.Conv_IntToString` (`KismetMathLibrary.FFloor` _currentsunlight)) "/" (`KismetStringLibrary.Conv_IntToString` (`KismetMathLibrary.FFloor` _maxsunlight))) (`self.Bars`))))))

(fn `Pause`
  (`GameplayStatics.SetGamePaused` true)
  (`UserWidget.AddToViewport` (`self.Pause Menu`) 0)
  (`Widget.RemoveFromParent` (`self.HUD`)))

(fn `Unpause`
  (`GameplayStatics.SetGamePaused` false)
  (`Widget.RemoveFromParent` (`self.Pause Menu`))
  (`UserWidget.AddToViewport` (`self.HUD`) 0))

(fn `UpdateAir`
  (if (> (`self.CurrentAir`) 0.0)
    (set `self.CurrentAir` (- (`self.CurrentAir`) (* (`GameplayStatics.GetGlobalTimeDilation`) (`self.AirDepletionRate`))))
    (set `/Game/UserInterface/Bars.AirPercentage` (/ (`self.CurrentAir`) (`self.MaxAir`)) (`self.Bars`))
    (set `/Game/UserInterface/Bars.AirText` (`KismetStringLibrary.Concat_StrStr` (`KismetStringLibrary.Conv_IntToString` (`KismetMathLibrary.FFloor` (`self.CurrentAir`))) "/" (`KismetStringLibrary.Conv_IntToString` (`KismetMathLibrary.FFloor` (`self.MaxAir`)))) (`self.Bars`))))

(fn `UpdateEnergy`
  (if (and (> (`self.CurrentAir`) 0.0) (> (`self.CurrentSunlight`) 0.0) (> (`self.CurrentWater`) 0.0) (< (`self.CurrentEnergy`) (`self.MaxEnergy`)))
    (set `self.CurrentEnergy` (+ 0.02 (`self.CurrentEnergy`)))
    (set `/Game/UserInterface/Bars.EnergyPercentage` (/ (`self.CurrentEnergy`) (`self.MaxEnergy`)) (`self.Bars`) :!label _label)
    (set `/Game/UserInterface/Bars.EnergyText` (`KismetStringLibrary.Concat_StrStr` (`KismetStringLibrary.Conv_IntToString` (`KismetMathLibrary.FFloor` (`self.CurrentEnergy`))) "/" (`KismetStringLibrary.Conv_IntToString` (`KismetMathLibrary.FFloor` (`self.MaxEnergy`)))) (`self.Bars`))
    (elif (> (`self.CurrentEnergy`) 0.0)
      (set `self.CurrentEnergy` (- (`self.CurrentEnergy`) (* (`GameplayStatics.GetGlobalTimeDilation`) (`self.EnergyDepletionRate`))))
      (goto _label))))

(fn `UpdateSunlight`
  (if (> (`self.CurrentSunlight`) 0.0)
    (set `self.CurrentSunlight` (- (`self.CurrentSunlight`) (* (`GameplayStatics.GetGlobalTimeDilation`) (`self.SunlightDepletionRate`))))
    (set `/Game/UserInterface/Bars.SunlightPercentage` (/ (`self.CurrentSunlight`) (`self.MaxSunlight`)) (`self.Bars`))
    (set `/Game/UserInterface/Bars.SunlightText` (`KismetStringLibrary.Concat_StrStr` (`KismetStringLibrary.Conv_IntToString` (`KismetMathLibrary.FFloor` (`self.CurrentSunlight`))) "/" (`KismetStringLibrary.Conv_IntToString` (`KismetMathLibrary.FFloor` (`self.MaxSunlight`)))) (`self.Bars`))))

(fn `UpdateWater`
  (if (> (`self.CurrentWater`) 0.0)
    (set `self.CurrentWater` (- (`self.CurrentWater`) (* (`GameplayStatics.GetGlobalTimeDilation`) (`self.WaterDepletionRate`))))
    (set `/Game/UserInterface/Bars.WaterPercentage` (/ (`self.CurrentWater`) (`self.MaxWater`)) (`self.Bars`))
    (set `/Game/UserInterface/Bars.WaterText` (`KismetStringLibrary.Concat_StrStr` (`KismetStringLibrary.Conv_IntToString` (`KismetMathLibrary.FFloor` (`self.CurrentWater`))) "/" (`KismetStringLibrary.Conv_IntToString` (`KismetMathLibrary.FFloor` (`self.MaxWater`)))) (`self.Bars`))))

(fn `UserConstructionScript`)