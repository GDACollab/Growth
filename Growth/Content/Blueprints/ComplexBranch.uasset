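; Compound branch actor that animates growth of five child-actor branches and then their leaves.
; BranchControl first scales the child actors up over about three seconds, using two size vectors for groups of three and two.
; It then spends about two seconds enlarging a shared leaf size, passed to each SingleBranch child through SingleBranchUpdate.
; Both phases use ForDelay, a timed loop macro stepping every 0.05 seconds.
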(event `BranchControl`
  (bind _leave_size (`self.leave size`))
  (`self.ForDelay` 3.0
    (:`LoopBody`
      (bind _output_get (set `self.Branch_0Size` (+ (`self.Branch_0Size`) (0.003 0.0 0.005))))
      (`SceneComponent.SetRelativeScale3D` (`self.ChildActor`) _output_get)
      (`SceneComponent.SetRelativeScale3D` (`self.ChildActor1`) _output_get)
      (`SceneComponent.SetRelativeScale3D` (`self.ChildActor2`) _output_get)
      (bind _output_get_2 (set `self.Branch_1Size` (+ (`self.Branch_1Size`) (0.003 0.0 0.005))))
      (`SceneComponent.SetRelativeScale3D` (`self.ChildActor3`) _output_get_2)
      (`SceneComponent.SetRelativeScale3D` (`self.ChildActor4`) _output_get_2))
    (:`Completed`
      (`self.ForDelay` 2.0
        (:`LoopBody`
          (bind _output_get_3 (set `self.leave size` (+ (stale _output_get_3) (0.00025 0.0 0.00025))))
          (bind _assingle_branch (cast `/Game/Blueprints/SingleBranch` (`ChildActorComponent.ChildActor` (`self.ChildActor`))))
          (`/Game/Blueprints/SingleBranch.SingleBranchUpdate` _assingle_branch _leave_size)
          (bind _assingle_branch_2 (cast `/Game/Blueprints/SingleBranch` (`ChildActorComponent.ChildActor` (`self.ChildActor1`))))
          (`/Game/Blueprints/SingleBranch.SingleBranchUpdate` _assingle_branch_2 _leave_size)
          (bind _assingle_branch_3 (cast `/Game/Blueprints/SingleBranch` (`ChildActorComponent.ChildActor` (`self.ChildActor2`))))
          (`/Game/Blueprints/SingleBranch.SingleBranchUpdate` _assingle_branch_3 _leave_size)
          (bind _assingle_branch_4 (cast `/Game/Blueprints/SingleBranch` (`ChildActorComponent.ChildActor` (`self.ChildActor3`))))
          (`/Game/Blueprints/SingleBranch.SingleBranchUpdate` _assingle_branch_4 _leave_size)
          (bind _assingle_branch_5 (cast `/Game/Blueprints/SingleBranch` (`ChildActorComponent.ChildActor` (`self.ChildActor4`))))
          (`/Game/Blueprints/SingleBranch.SingleBranchUpdate` _assingle_branch_5 _leave_size))))))

(event `Update_leave_1`)

(fn `UserConstructionScript`)