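; SingleBranch is a branch Blueprint that controls the size of fifteen Paper2D sprites, apparently its leaves.
; The SingleBranchUpdate event applies the passed LeaveSize as relative scale to all the sprites at once.
; A ForDelay macro provides a timed loop stepping every 0.05 seconds over a given duration, but no graph here calls it.
; Update_leave_1 and the construction script are empty.
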(event `SingleBranchUpdate`
  (params (Leave_size :type "Vector Structure"))
  (`SceneComponent.SetRelativeScale3D` (`self.PaperSprite`) Leave_size)
  (`SceneComponent.SetRelativeScale3D` (`self.PaperSprite1`) Leave_size)
  (`SceneComponent.SetRelativeScale3D` (`self.PaperSprite2`) Leave_size)
  (`SceneComponent.SetRelativeScale3D` (`self.PaperSprite3`) Leave_size)
  (`SceneComponent.SetRelativeScale3D` (`self.PaperSprite4`) Leave_size)
  (`SceneComponent.SetRelativeScale3D` (`self.PaperSprite5`) Leave_size)
  (`SceneComponent.SetRelativeScale3D` (`self.PaperSprite6`) Leave_size)
  (`SceneComponent.SetRelativeScale3D` (`self.PaperSprite7`) Leave_size)
  (`SceneComponent.SetRelativeScale3D` (`self.PaperSprite8`) Leave_size)
  (`SceneComponent.SetRelativeScale3D` (`self.PaperSprite9`) Leave_size)
  (`SceneComponent.SetRelativeScale3D` (`self.PaperSprite10`) Leave_size)
  (`SceneComponent.SetRelativeScale3D` (`self.PaperSprite11`) Leave_size)
  (`SceneComponent.SetRelativeScale3D` (`self.PaperSprite12`) Leave_size)
  (`SceneComponent.SetRelativeScale3D` (`self.PaperSprite13`) Leave_size)
  (`SceneComponent.SetRelativeScale3D` (`self.PaperSprite14`) Leave_size))

(event `Update_leave_1`)

(fn `UserConstructionScript`)