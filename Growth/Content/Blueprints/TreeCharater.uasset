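; Growable sprite-based tree actor that also creates the button and menu widgets and shows the mouse cursor.
; On BeginPlay it spawns a root actor and attaches it to one of three sprite sockets at random.
; UpdateTree uses a timed ForDelay loop to scale the sprite while TreeGrowth is set.
; When the loop completes, it clears that flag and calls BranchControl on four ComplexBranch child actors.
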(event `self.ReceiveBeginPlay`
  ;[1 1 1] Widget Initialization
  (`|ExecutionSequence`
    (:`then_0`
      (bind _returnvalue (`|CreateWidget` "/Game/Blueprints/BP_Button.BP_Button_C"))
      (`UserWidget.AddToViewport` _returnvalue 0)
      (set `PlayerController.bShowMouseCursor` true (`GameplayStatics.GetPlayerController` 0))
      ;[1 1 1] Randomly generate root sprite on one of three sockets
      (bind _returnvalue_2 (`|SpawnActorFromClass` "/Game/Blueprints/Root_BP.Root_BP_C" (`KismetMathLibrary.MakeTransform` (0.0 5.0 -15.0) (struct) (0.5 0.5 0.5)) "AdjustIfPossibleButDontSpawnIfColliding" "OverrideRootScale"))
      (switch `int` (`KismetMathLibrary.RandomInteger` 3)
        (:`0`
          (bind _defaultsceneroot (`/Game/Blueprints/Root_BP.DefaultSceneRoot` _returnvalue_2))
          (`SceneComponent.K2_AttachTo` _defaultsceneroot (`self.Sprite`) "LeftRoot" "KeepRelativeOffset" true))
        (:`1`
          (`SceneComponent.K2_AttachTo` _defaultsceneroot (`self.Sprite`) "MidRoot" "KeepRelativeOffset" true))
        (:`2`
          (`SceneComponent.K2_AttachTo` _defaultsceneroot (`self.Sprite`) "RightRoot" "KeepRelativeOffset" true))))
    (:`then_1`
      (bind _returnvalue_3 (`|CreateWidget` "/Game/Blueprints/Menu_Button.Menu_Button_C"))
      (`UserWidget.AddToViewport` _returnvalue_3 0))))

(event `UpdateTree`
  ;[1 1 1] Growth Control
  (`self.ForDelay` 3.0
    (:`LoopBody`
      (if (`self.Tree_Growth`)
        (bind _output_get (set `self.Tree_Scale` (+ (`self.Tree_Scale`) (0.005 0.0 0.005))))
        (`SceneComponent.SetRelativeScale3D` (`self.Sprite`) _output_get)))
    (:`Completed`
      (set `self.Tree_Growth` false)
      (bind _ascomplex_branch (cast `/Game/Blueprints/ComplexBranch` (`ChildActorComponent.ChildActor` (`self.complexbranch`))))
      (`/Game/Blueprints/ComplexBranch.BranchControl` _ascomplex_branch)
      (bind _ascomplex_branch_2 (cast `/Game/Blueprints/ComplexBranch` (`ChildActorComponent.ChildActor` (`self.complexbranch1`))))
      (`/Game/Blueprints/ComplexBranch.BranchControl` _ascomplex_branch_2)
      (bind _ascomplex_branch_3 (cast `/Game/Blueprints/ComplexBranch` (`ChildActorComponent.ChildActor` (`self.complexbranch2`))))
      (`/Game/Blueprints/ComplexBranch.BranchControl` _ascomplex_branch_3)
      (bind _ascomplex_branch_4 (cast `/Game/Blueprints/ComplexBranch` (`ChildActorComponent.ChildActor` (`self.complexbranch3`))))
      (`/Game/Blueprints/ComplexBranch.BranchControl` _ascomplex_branch_4))))

(event `Update_leave_1`)

(fn `UserConstructionScript`)