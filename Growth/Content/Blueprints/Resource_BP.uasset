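; Draggable resource pickup, labeled Water, Air or Sunlight by its type, that the player drops on the tree to collect.
; Clicking makes it follow the mouse each tick with a swept move, using cursor deprojection scaled by the player controller's Y and flattened to Y=0.
; Releasing it during any actor overlap, with no tree-specific check, increments that resource on the first GrowthCamera found and destroys the pickup.
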(event `self.ReceiveBeginPlay`
  ;[1 0.1037 0.6335] Get Reference to Camera
  (bind _output_get (set `self.CameraController` (`GameplayStatics.GetPlayerController` 0)))
  (`self.EnableInput` _output_get)
  ;[1 1 1] Set Resource Text
  (switch `/Game/Blueprints/Enum_ResourceType` (`self.ResourceType`)
    (:`NewEnumerator0`
      (`TextRenderComponent.K2_SetText` (`self.TextComponent`) (`KismetTextLibrary.Conv_StringToText` "Water")))
    (:`NewEnumerator1`
      (`TextRenderComponent.K2_SetText` (`self.TextComponent`) (`KismetTextLibrary.Conv_StringToText` "Air")))
    (:`NewEnumerator2`
      (`TextRenderComponent.K2_SetText` (`self.TextComponent`) (`KismetTextLibrary.Conv_StringToText` "Sunlight")))))

(event `self.ReceiveActorEndOverlap`
  (params (OtherActor :type "Actor Object Reference"))
  ;[1 1 1] Destroy resource when dropped on tree
  (set `self.Overlap` false))

(event `self.ReceiveActorBeginOverlap`
  (params (OtherActor :type "Actor Object Reference"))
  ;[1 1 1] Destroy resource when dropped on tree
  (set `self.Overlap` true))

(event `self.ReceiveActorOnClicked`
  ;[1 1 1] EnableMouseFollowOnDrag
  (set `self.FollowMouse` true))

(event `self.ReceiveActorOnReleased`
  ;[1 1 1] EnableMouseFollowOnDrag
  (set `self.FollowMouse` false)
  ;[1 1 1] Destroy resource when dropped on tree
  (if (`self.Overlap`)
    (bind _outactors (`GameplayStatics.GetAllActorsOfClass` "/Game/Blueprints/Player/GrowthCamera.GrowthCamera_C"))
    (`/Game/Blueprints/Player/GrowthCamera.IncrementResource` (`KismetArrayLibrary.Array_Get` _outactors) (`self.ResourceType`))
    (`self.K2_DestroyActor`)))

(event `InputAction|Click`
  (params (Key :type "Key Structure" :default "AnyKey"))
  ;[1 1 1] EnableMouseFollowOnDrag
  (:`Released`
    (set `self.FollowMouse` false)))

(event `self.ReceiveTick`
  (params (DeltaSeconds :type "Float (single-precision)"))
  ;[1 1 1] FollowMouseOnDrag
  (if (`self.FollowMouse`)
    (bind _returnvalue (`self.GetMousePosition`))
    (`self.K2_SetActorLocation` _returnvalue true)))

(fn `GetMousePosition`
  (returns (ReturnValue :type "Vector Structure"))
  (bind (_worldlocation _worlddirection) (`PlayerController.DeprojectMousePositionToWorld` (`self.CameraController`)))
  (return (`KismetMathLibrary.MakeVector` (.x (+ _worldlocation (* _worlddirection (.y (`self.K2_GetActorLocation` (`self.CameraController`)))))) 0.0 (.z (+ _worldlocation (* _worlddirection (.y (`self.K2_GetActorLocation` (`self.CameraController`)))))))))

(fn `UserConstructionScript`)